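; Spawner actor that repeatedly spawns an actor at random positions on a fixed-Y plane.
; Tick re-rolls an integer delay of a few seconds every frame and feeds it to a Delay, whose pending countdown paces the spawns.
; When the Delay completes, a helper picks random X and Z coordinates, which become the transform for SpawnActor; no actor class is shown.
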(event `self.ReceiveTick`
  (params (DeltaSeconds :type "Float (single-precision)"))
  (`self.set_random_number`)
  (`KismetSystemLibrary.Delay` (`KismetMathLibrary.Conv_IntToDouble` (`self.spawn_delay`)))
  (`self.set_random_coord`)
  (`|SpawnActorFromClass` "/Game/Character/Deer.Deer_C" (`KismetMathLibrary.Conv_VectorToTransform` (`self.map_coord`)) "Undefined" "OverrideRootScale" null null))

(fn `set_random_coord`
  (set `self.map_coord` (`KismetMathLibrary.MakeVector` (`KismetMathLibrary.Conv_IntToDouble` (`KismetMathLibrary.RandomIntegerInRange` 0 1000)) 20.0 (`KismetMathLibrary.Conv_IntToDouble` (`KismetMathLibrary.RandomIntegerInRange` -1000)))))

(fn `set_random_number`
  (set `self.spawn_delay` (`KismetMathLibrary.RandomIntegerInRange` 1 5)))

(fn `UserConstructionScript`)